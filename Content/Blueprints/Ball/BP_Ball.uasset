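; BP_Ball is a team-owned ball that knocks back and damages tanks of the opposing team.
; SetTeam records the owning team and swaps the mesh material to match.
; When its sphere overlaps a BP_Tank on another team, it pushes the tank away with an impulse scaled by ball speed.
; Above a minimum speed, it also applies damage proportional to that speed.
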(event OnComponentBeginOverlap(Sphere)
  (params (OverlappedComponent :type Primitive%20Component%20Object%20Reference) (OtherActor :type Actor%20Object%20Reference) (OtherComp :type Primitive%20Component%20Object%20Reference) (OtherBodyIndex :type Integer) (bFromSweep :type Boolean) (SweepResult :type Hit%20Result%20Structure%20%28by%20ref%29))
  (bind _returnvalue (Transformation|GetVelocity))
  (bind _returnvalue_2 (Math|Vector|VectorLength _returnvalue))
  ;[1 1 1] Collision with tank
  (bind _asbp_tank (Utilities|Casting|CastToBP_Tank OtherActor))
  ;;[1 1 1] If tank is not part of current team
  (if (!= (Variables|Default|GetBallOwner) (Variables|/Game/Blueprints/Tank/BP/BP_Tank.BP_Tank_C|GetTeam _asbp_tank))
    ;;[1 1 1] Add force
    (Physics|AddImpulse (Variables|/Script/PhysXVehicles.WheeledVehicle|GetMesh _asbp_tank) (* (- (Transformation|GetActorLocation OtherActor) (Transformation|GetActorLocation)) (* _returnvalue_2 1.5)) "None" false)
    ;;[1 1 1] Apply Damage
    (if (>= _returnvalue_2 1e+02)
      (Game|Damage|ApplyDamage _asbp_tank (/ _returnvalue_2 1e+02) 0 0))))

(event Custom|SetTeam
  (params (BallOwner :type Teams%20Enum :default "NewEnumerator0"))
  ;[1 1 1] Set Material to show team
  (bind _output_get (Variables|Default|SetBallOwner BallOwner))
  (Rendering|Material|SetMaterial (Variables|Default|GetMesh) 0 (Utilities|Select :Index _output_get :NewEnumerator0 "/Game/Vehicle/Sedan/Materials/M_Vehicle_Sedan.M_Vehicle_Sedan" :NewEnumerator1 "/AnimationSharing/AnimSharingRed.AnimSharingRed")))

(fn ConstructionScript)