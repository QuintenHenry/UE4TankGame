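; Game mode for a team tank-and-ball match, handling teams, spawning, scoring and the win condition.
; BeginPlay sets UI-only input and puts the first AI tank on one team, the rest on the other.
; Spawn resets the ball and places tanks at randomized team-tagged PlayerStarts, briefly frozen; RespawnPlayer restores one tank's health and position.
; AddPoint calls Spawn until a team reaches the target, then shows the player's win state.
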(event Custom|Spawn
  ;[1 1 1] Spawn all players and ball
  (Variables|Default|SetOffset (Math|Random|RandomIntegerinRange 0 1)) ; randomize position
  (bind _outactors (Actor|GetAllActorsOfClass "/Game/Blueprints/Tank/BP/BP_Tank.BP_Tank_C"))
  (for (_array_element _array_index) _outactors
    ;;[1 1 1] Spawn player
    (Variables|/Game/Blueprints/Tank/BP/BP_Tank.BP_Tank_C|SetCanMove _array_element false)
    (bind _outactors_2 (Actor|GetAllActorsOfClasswithTag "/Script/Engine.PlayerStart" (Utilities|String|StringToName (Utilities|String|EnumtoString (Variables|/Game/Blueprints/Tank/BP/BP_Tank.BP_Tank_C|GetTeam _array_element)))))
    (Transformation|SetActorTransform _array_element (Math|Transform|MakeTransform (Transformation|GetActorLocation (Utilities|Array|Get(acopy) _outactors_2 (Math|Integer|%(Integer) (+ _array_index (Variables|Default|GetOffset)) 2))) (Math|Rotator|FindLookatRotation (Transformation|GetActorLocation (Utilities|Array|Get(acopy) _outactors_2 (Math|Integer|%(Integer) (+ _array_index (Variables|Default|GetOffset)) 2))) (Math|Vector|MakeVector 0.0 0.0 0.0))) false true))
  ;;[1 1 1] Spawn ball
  (bind _returnvalue (Actor|GetActorOfClass "/Game/Blueprints/Ball/BP_Ball.BP_Ball_C"))
  (Transformation|SetActorLocation _returnvalue "0, 0,500.000000" false true)
  ;;[1 1 1] Reset ball velocity
  (Class|PrimitiveComponent|SetAllPhysicsAngularVelocityinDegrees (Variables|/Game/Blueprints/Ball/BP_Ball.BP_Ball_C|GetMesh _returnvalue) (Math|Vector|MakeVector 0.0 0.0 0.0) false)
  (Class|PrimitiveComponent|SetAllPhysicsLinearVelocity (Variables|/Game/Blueprints/Ball/BP_Ball.BP_Ball_C|GetMesh _returnvalue) "0, 0, 0" false)
  ;;[1 1 1] Let everyone move after 3 seconds
  (Utilities|FlowControl|Delay 3.0)
  (bind _outactors_3 (Actor|GetAllActorsOfClass "/Game/Blueprints/Tank/BP/BP_Tank.BP_Tank_C"))
  (for _array_element_2 _outactors_3
    (Variables|/Game/Blueprints/Tank/BP/BP_Tank.BP_Tank_C|SetCanMove _array_element_2 true)))

(event Custom|RespawnPlayer
  (params (Target :type BP%20Tank%20Object%20Reference))
  ;[1 1 1] Spawn player
  (Variables|/Game/Blueprints/Tank/BP/BP_Tank.BP_Tank_C|SetHealth Target 1e+02)
  (Variables|/Game/Blueprints/Tank/BP/BP_Tank.BP_Tank_C|SetCanMove Target false)
  (bind _outactors (Actor|GetAllActorsOfClasswithTag "/Script/Engine.PlayerStart" (Utilities|String|StringToName (Utilities|String|EnumtoString (Variables|/Game/Blueprints/Tank/BP/BP_Tank.BP_Tank_C|GetTeam Target)))))
  (Transformation|SetActorTransform Target (Math|Transform|MakeTransform (Transformation|GetActorLocation (Utilities|Array|Get(acopy) _outactors)) (Math|Rotator|FindLookatRotation (Transformation|GetActorLocation (Utilities|Array|Get(acopy) _outactors)) (Math|Vector|MakeVector 0.0 0.0 0.0))) false true)
  (Utilities|FlowControl|Delay 3.0)
  (Variables|/Game/Blueprints/Tank/BP/BP_Tank.BP_Tank_C|SetCanMove Target true))

(event EventBeginPlay
  (bind _returnvalue (Game|GetPlayerController 0))
  ;[1 1 1] Begin
  (Variables|/Script/Engine.PlayerController|SetbShowMouseCursor _returnvalue true)
  (Input|SetInputModeUIOnly _returnvalue 0 "DoNotLock")
  (bind _outactors (Actor|GetAllActorsOfClass "/Game/Blueprints/Tank/AI/BP_TankAI.BP_TankAI_C"))
  (for (_array_element _array_index) _outactors
    (if (== _array_index 0)
      (Variables|/Game/Blueprints/Tank/BP/BP_Tank.BP_Tank_C|SetTeam _array_element "NewEnumerator0")
      (else
        (Variables|/Game/Blueprints/Tank/BP/BP_Tank.BP_Tank_C|SetTeam _array_element "NewEnumerator1")))))

(fn ConstructionScript)

(fn AddPoint
  (params (Team :type Teams%20Enum :default "NewEnumerator0"))
  (bind _returnvalue (Math|Conversions|ToInteger(Byte) Team))
  (bind _points (Variables|Default|GetPoints))
  (bind _output (Utilities|Array|Get(acopy) _points _returnvalue))
  ;[1 1 1] Add point
  (|SetBy-RefVar _output (+ _output 1))
  ;[1 1 1] Win game after 3 or more points
  (if (>= _output (Variables|Default|GetPointsRequiredToWin))
    (bind _asbp_tank (Utilities|Casting|CastToBP_Tank (Game|Player|GetPlayerPawn 0)))
    (Variables|/Game/Blueprints/Tank/BP/BP_Tank.BP_Tank_C|SetCanMove _asbp_tank false)
    (Variables|/Script/Engine.PlayerController|SetbShowMouseCursor (Game|GetPlayerController 0) true)
    (Default|SetWinState (Variables|/Game/Blueprints/Tank/BP/BP_Tank.BP_Tank_C|GetPlayerWidget _asbp_tank) (Utilities|Enum|Equal(Enum) Team "NewEnumerator0"))
    (else
      ;[1 1 1] Respawn
      (CallFunction|Spawn))))